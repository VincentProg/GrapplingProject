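; Player character Blueprint with two independent grappling hooks that pull its physics Body toward hooked points.
; Right mouse fires the left hook and left mouse the right, using forward object traces from Body; releasing resets that hook.
; Tick interpolates each visible grapple line toward its hit point until close.
; Mouse wheel down then adds velocity toward each attached point, scaled by distance and frame time.
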(event `self.ReceiveTick`
  (params (DeltaSeconds :type "Float (single-precision)"))
  ;[0 1 0.01725] Event Tick
  (`|ExecutionSequence`
    (:`then_0`
      (if (`self.HookedLeft`)
        (if (not (`self.HookLeftMoveFinished`))
          (bind _reachedlocation (`self.MoveLeftRope`))
          (set `self.HookLeftMoveFinished` _reachedlocation))))
    (:`then_1`
      (if (`self.HookedRight`)
        (if (not (`self.HookRightMoveFinished`))
          (bind _reachedlocation_2 (`self.MoveRightRope`))
          (set `self.HookRightMoveFinished` _reachedlocation_2))))))

(event `Key|RightMouseButton`
  (params (Key :type "Key Structure"))
  (bind _body (`self.Body`))
  (bind _returnvalue (`SceneComponent.K2_GetComponentLocation` _body))
  ;[0 0.3529 1] Grappling LEFT
  (:`Pressed`
    (bind (_outhit _returnvalue_2) (`KismetSystemLibrary.LineTraceSingleForObjects` :`Start` _returnvalue :`End` (+ (* (`SceneComponent.GetForwardVector` _body) 5000.0) _returnvalue) :`ObjectTypes` (`|MakeArray` "ObjectTypeQuery1" "ObjectTypeQuery2" :!type "EObjectTypeQuery Enum") :`DrawDebugType` "ForDuration"))
    (if _returnvalue_2
      (set `self.HookedLeft` true)
      (set `self.HookLeftLocation` (`.Location` (`GameplayStatics.BreakHitResult` _outhit)))
      (else
        (`self.StopLEFTGrapple`))))
  (:`Released`
    (`self.StopLEFTGrapple`)))

(event `Key|LeftMouseButton`
  (params (Key :type "Key Structure"))
  (bind _body (`self.Body`))
  (bind _returnvalue (`SceneComponent.K2_GetComponentLocation` _body))
  ;[1 0.3779 0] Grappling LEFT
  (:`Pressed`
    (bind (_outhit _returnvalue_2) (`KismetSystemLibrary.LineTraceSingleForObjects` :`Start` _returnvalue :`End` (+ (* (`SceneComponent.GetForwardVector` _body) 5000.0) _returnvalue) :`ObjectTypes` (`|MakeArray` "ObjectTypeQuery1" "ObjectTypeQuery2" :!type "EObjectTypeQuery Enum") :`DrawDebugType` "ForDuration"))
    (if _returnvalue_2
      (set `self.HookedRight` true)
      (set `self.HookRightLocation` (`.Location` (`GameplayStatics.BreakHitResult` _outhit)))
      (else
        (`self.StopRIGHTGrapple`))))
  (:`Released`
    (`self.StopRIGHTGrapple`)))

(event `StopLEFTGrapple`
  (bind _grapplelineleft (`self.GrappleLineLeft`))
  ;[0 0.3529 1] Stop LEFT Grapple
  (set `self.HookedLeft` false)
  (set `self.HookLeftMoveFinished` false)
  (`SceneComponent.SetVisibility` _grapplelineleft false false)
  (`SceneComponent.K2_SetWorldLocation` _grapplelineleft (0.0 0.0 0.0) false false))

(event `StopRIGHTGrapple`
  (bind _grapplelineright (`self.GrappleLineRight`))
  ;[1 0.3779 0] Stop RIGHT Grapple
  (set `self.HookedRight` false)
  (set `self.HookRightMoveFinished` false)
  (`SceneComponent.SetVisibility` _grapplelineright false false)
  (`SceneComponent.K2_SetWorldLocation` _grapplelineright (0.0 0.0 0.0) false false))

(event `Key|MouseScrollDown`
  (params (Key :type "Key Structure"))
  (bind _grapplelineleft (`self.GrappleLineLeft`))
  (bind _grapplelineright (`self.GrappleLineRight`))
  ;[1 0 0.9183] Move Grapple Player
  (:`Pressed`
    (`|ExecutionSequence`
      (:`then_0`
        (if (`self.HookedLeft`)
          (if (`self.HookLeftMoveFinished`)
            (`self.MoveLeftGrapplePlayer`)
            (`SceneComponent.K2_SetWorldLocation` _grapplelineleft (`KismetMathLibrary.VInterpTo` (`SceneComponent.K2_GetComponentLocation` _grapplelineleft) (`self.HookLeftLocation`) (`GameplayStatics.GetWorldDeltaSeconds`) 250.0) false false))))
      (:`then_1`
        (if (`self.HookedRight`)
          (if (`self.HookRightMoveFinished`)
            (`self.MoveRightGrapplePlayer`)
            (`SceneComponent.K2_SetWorldLocation` _grapplelineright (`KismetMathLibrary.VInterpTo` (`SceneComponent.K2_GetComponentLocation` _grapplelineright) (`self.HookRightLocation`) (`GameplayStatics.GetWorldDeltaSeconds`) 250.0) false false)))))))

(fn `MoveLeftGrapplePlayer`
  (`PrimitiveComponent.SetPhysicsLinearVelocity` (`self.Body`) (* (- (`self.HookLeftLocation`) (`SceneComponent.K2_GetComponentLocation` (`self.Body`))) (* (`GameplayStatics.GetWorldDeltaSeconds`) 50.0)) true "None"))

(fn `MoveLeftRope`
  (returns (ReachedLocation :type Boolean))
  (bind _grapplelineleft (`self.GrappleLineLeft`))
  (bind _hookleftlocation (`self.HookLeftLocation`))
  (bind _returnvalue (`SceneComponent.K2_GetComponentLocation` _grapplelineleft))
  (`SceneComponent.SetVisibility` _grapplelineleft true false)
  (if (<= (`KismetMathLibrary.VSize` (- _returnvalue _hookleftlocation)) 100.0)
    (return true)
    (else
      (`SceneComponent.K2_SetWorldLocation` _grapplelineleft (`KismetMathLibrary.VInterpTo` _returnvalue _hookleftlocation (`GameplayStatics.GetWorldDeltaSeconds`) 35.0) false false)
      (return false))))

(fn `MoveRightGrapplePlayer`
  (`PrimitiveComponent.SetPhysicsLinearVelocity` (`self.Body`) (* (- (`self.HookRightLocation`) (`SceneComponent.K2_GetComponentLocation` (`self.Body`))) (* (`GameplayStatics.GetWorldDeltaSeconds`) 50.0)) true "None"))

(fn `MoveRightRope`
  (returns (ReachedLocation :type Boolean))
  (bind _grapplelineright (`self.GrappleLineRight`))
  (bind _hookrightlocation (`self.HookRightLocation`))
  (bind _returnvalue (`SceneComponent.K2_GetComponentLocation` _grapplelineright))
  (`SceneComponent.SetVisibility` _grapplelineright true false)
  (if (<= (`KismetMathLibrary.VSize` (- _returnvalue _hookrightlocation)) 100.0)
    (return true)
    (else
      (`SceneComponent.K2_SetWorldLocation` _grapplelineright (`KismetMathLibrary.VInterpTo` _returnvalue _hookrightlocation (`GameplayStatics.GetWorldDeltaSeconds`) 35.0) false false)
      (return false))))

(fn `UserConstructionScript`)